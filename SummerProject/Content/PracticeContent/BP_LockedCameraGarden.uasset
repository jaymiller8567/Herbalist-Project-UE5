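; Practice Blueprint for a garden scene that makes a flower pot respond to mouse interaction.
; Component-bound cursor events print a debug message on hover, and on click print a message and swap the pot's first material slot to a buildings texture material.
; The default BeginPlay, overlap and Tick events are disabled, and the construction script only calls its parent.
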(event OnBeginCursorOver(flower_pot)
  (params (TouchedComponent :type Primitive%20Component%20Object%20Reference))
  (Development|PrintString "Hovered over pot!"))

(event OnClicked(flower_pot)
  (params (TouchedComponent :type Primitive%20Component%20Object%20Reference) (ButtonPressed :type Key%20Structure :default "None"))
  (Development|PrintString "Clicked!")
  (Rendering|Material|SetMaterial (Variables|Default|Getflower_pot) 0 "/Game/dae-end-assignment-grandmas-house/source/BuildingsDoorsRidgeends_01_tex.BuildingsDoorsRidgeends_01_tex"))

(event EventBeginPlay
  (|CallParentFunction) ; This node is disabled and will not be called.\nDrag off pins to build functionality.
)

(event Collision|EventActorBeginOverlap
  (params (OtherActor :type Actor%20Object%20Reference))
  (|CallParentFunction OtherActor) ; This node is disabled and will not be called.\nDrag off pins to build functionality.
)

(event EventTick
  (params (DeltaSeconds :type Float%20%28single-precision%29))
  (|CallParentFunction DeltaSeconds) ; This node is disabled and will not be called.\nDrag off pins to build functionality.
)

(fn ConstructionScript
  (|CallParentFunction))