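; A trigger actor that locks the player's view to a fixed camera when BP_FirstPerson_Collector overlaps it.
; On overlap it saves the current camera rotation and blends the view target to the actor that owns ViewPoint.
; While locked, the IA_OpenMail input blends back to the player pawn and resets the first-person camera to a fixed relative location.
; The saved world rotation is reapplied as the camera's relative rotation.
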(event Input|EnhancedActionEvents|EnhancedInputActionIA_OpenMail
  (params (ActionValue :type Boolean) (ElapsedSeconds :type Float%20%28double-precision%29) (TriggeredSeconds :type Float%20%28double-precision%29) (InputAction :type Input%20Action%20Object%20Reference :default "/Game/PracticeContent/Mail/IA_OpenMail.IA_OpenMail"))
  (bind _returnvalue (Game|Player|GetPlayerPawn 0))
  (bind _playercamrotation (Variables|Default|GetPlayerCamRotation))
  (if (Variables|Default|GetisLockedCam)
    (bind _asbp_first_person_collector (Utilities|Casting|CastToBP_FirstPerson_Collector _returnvalue))
    (Game|Player|SetViewTargetwithBlend (Game|GetPlayerController 0) _asbp_first_person_collector 0.5 "VTBlend_Linear" 0.0 false)
    (bind _asbp_first_person_collector_2 (Utilities|Casting|CastToBP_FirstPerson_Collector _returnvalue))
    (Transformation|SetRelativeRotation (Variables|/Game/FirstPerson/Blueprints/BP_FirstPersonCharacter.BP_FirstPersonCharacter_C|GetFirstPersonCamera _asbp_first_person_collector_2) _playercamrotation false false)
    (Development|PrintString (Utilities|String|ToString(Rotator) _playercamrotation))
    (Transformation|SetRelativeLocation (Variables|/Game/FirstPerson/Blueprints/BP_FirstPersonCharacter.BP_FirstPersonCharacter_C|GetFirstPersonCamera _asbp_first_person_collector_2) "-10.000000,0.000000,60.000000" false false)
    (Variables|Default|SetisLockedCam false)))

(event EventBeginPlay)

(event Collision|EventActorBeginOverlap
  (params (OtherActor :type Actor%20Object%20Reference))
  (Utilities|Casting|CastToBP_FirstPerson_Collector OtherActor
    (:then
      (bind _output_get (Variables|Default|SetPlayerController (Game|GetPlayerController 0)))
      (Variables|Default|SetPlayerCamRotation (Camera|GetCameraRotation (Variables|/Script/Engine.PlayerController|GetPlayerCameraManager _output_get)))
      (Game|Player|SetViewTargetwithBlend _output_get (Components|GetOwner (Variables|Default|GetViewPoint)) 0.5 "VTBlend_Linear" 0.0 false)
      (Variables|Default|SetisLockedCam true))
    (:CastFailed
      (Development|PrintString "Cast Failed!"))))

(event EventTick
  (params (DeltaSeconds :type Float%20%28single-precision%29)))

(fn ConstructionScript)