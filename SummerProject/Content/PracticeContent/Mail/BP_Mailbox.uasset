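; BP_Mailbox is an interactable mailbox that the player can open while standing at it.
; Actor overlap events toggle an AtMailbox flag, reacting only to BP_FirstPerson_Collector.
; When IA_Interact completes with that flag set, it broadcasts OnMailboxOpen, leaving the response to bound listeners.
; Debug prints report the approach and each interact press; PlayerInput is set true just before its check, so only AtMailbox gates opening.
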(event Input|EnhancedActionEvents|EnhancedInputActionIA_Interact
  (params (ActionValue :type Boolean) (ElapsedSeconds :type Float%20%28double-precision%29) (TriggeredSeconds :type Float%20%28double-precision%29) (InputAction :type Input%20Action%20Object%20Reference :default "/Game/FirstPerson/Input/Actions/IA_Interact.IA_Interact"))
  (:Completed
    (bind _output_get (Variables|Default|SetplayerInput true))
    (if (and _output_get (Variables|Default|GetatMailbox))
      (Development|PrintString "Pressed U while inside box")
      (Default|CallOnMailboxOpen)
      (else
        (Development|PrintString "Pressed U not inside box")))))

(event EventBeginPlay)

(event Collision|EventActorBeginOverlap
  (params (OtherActor :type Actor%20Object%20Reference))
  (Utilities|Casting|CastToBP_FirstPerson_Collector OtherActor)
  (Development|PrintString "Player approached the mailbox!")
  (Variables|Default|SetatMailbox true))

(event EventTick
  (params (DeltaSeconds :type Float%20%28single-precision%29)))

(event Collision|EventActorEndOverlap
  (params (OtherActor :type Actor%20Object%20Reference))
  (Utilities|Casting|CastToBP_FirstPerson_Collector OtherActor)
  (Variables|Default|SetatMailbox false))

(fn ConstructionScript)