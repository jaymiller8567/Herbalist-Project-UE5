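; BP_LockedCameraGarden is a gardening actor that groups child planters and has a ViewPoint component, apparently for a fixed-camera garden view.
; SetUpPlanters collects its BP_Planter child actors into PlanterActors, though nothing in these graphs calls it.
; The construction script only logs ViewPoint's child components.
; Disconnected leftover nodes would gather BP_Plant actors from each planter, and no camera logic is present.
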(fn ConstructionScript
  (for _array_element (Components|GetChildrenComponents (Variables|Default|GetViewPoint) false)
    (Development|PrintText (Utilities|Text|ToText(Object) _array_element) false)))

(fn SetUpPlanters
  (for _array_element (Actor|GetAllChildActors false)
    (bind _asbp_planter (Utilities|Casting|CastToBP_Planter _array_element))
    (Utilities|IsValid _asbp_planter
      (:Is%20Valid
        (Utilities|Array|Add (Variables|Default|GetPlanterActors) _asbp_planter)))))