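; BP_Planter is a clickable planter actor for a gardening feature, with a pot mesh and a plant mesh.
; The construction script sets the plant mesh through CollapseGraph, fed by the Plant variable.
; Cursor events toggle a highlight material on the pot via PlanterHover.
; A click prints a debug message, swaps the pot material and sets Clicked, which stops further hover changes.
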(event OnClicked(Planter)
  (params (TouchedComponent :type Primitive%20Component%20Object%20Reference) (ButtonPressed :type Key%20Structure :default "None"))
  (CallFunction|PlanterClicked))

(event OnBeginCursorOver(Planter)
  (params (TouchedComponent :type Primitive%20Component%20Object%20Reference))
  (Variables|Default|SetHovered true)
  (CallFunction|PlanterHover))

(event OnEndCursorOver(Planter)
  (params (TouchedComponent :type Primitive%20Component%20Object%20Reference))
  (Variables|Default|SetHovered false)
  (CallFunction|PlanterHover))

(event EventBeginPlay)

(event Collision|EventActorBeginOverlap
  (params (OtherActor :type Actor%20Object%20Reference)))

(event EventTick
  (params (DeltaSeconds :type Float%20%28single-precision%29)))

(fn ConstructionScript
  (Components|StaticMesh|SetStaticMesh (Variables|Default|GetPlantModel) (|CollapseGraph (Variables|Default|GetPlant))))

(fn PlanterClicked
  (Development|PrintString "Clicked!")
  (Rendering|Material|SetMaterial (Variables|Default|GetPlanter) 0 "/Game/dae-end-assignment-grandmas-house/source/BuildingsDoorsRidgeends_01_tex.BuildingsDoorsRidgeends_01_tex")
  (Variables|Default|SetClicked true))

(fn PlanterHover
  (bind _planter (Variables|Default|GetPlanter))
  (if (not (Variables|Default|GetClicked))
    (if (Variables|Default|GetHovered)
      (Rendering|Material|SetMaterial _planter 0 "/Game/Materials/Select.Select")
      (else
        (Rendering|Material|SetMaterial _planter 0 "/Game/Materials/pot_Mat.pot_Mat")))))