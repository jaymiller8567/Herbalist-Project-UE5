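; BP_Garden is a gardening actor that keeps a Planters list of the BP_Planter child actors attached to it.
; Its Construction Script calls SetUpPlanters when that list is shorter than the count of all descendant child actors.
; SetUpPlanters clears the list and refills it uniquely from direct children only.
; The event graph is empty, and a nested loop collecting BP_Plant actors from the planters is left disconnected.
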(event EventBeginPlay)

(event Collision|EventActorBeginOverlap
  (params (OtherActor :type Actor%20Object%20Reference)))

(event EventTick
  (params (DeltaSeconds :type Float%20%28single-precision%29)))

(fn ConstructionScript
  (if (< (Utilities|Array|Length (Variables|Default|GetPlanters)) (Utilities|Array|Length (Actor|GetAllChildActors true)))
    (CallFunction|SetUpPlanters)))

(fn SetUpPlanters
  (Utilities|Array|Clear (Variables|Default|GetPlanters))
  (for _array_element (Actor|GetAllChildActors false)
    (bind _asbp_planter (Utilities|Casting|CastToBP_Planter _array_element))
    (Utilities|IsValid _asbp_planter
      (:Is%20Valid
        (Utilities|Array|AddUnique (Variables|Default|GetPlanters) _asbp_planter))
      (:Is%20Not%20Valid
        (Development|PrintText "Invalid!")))))