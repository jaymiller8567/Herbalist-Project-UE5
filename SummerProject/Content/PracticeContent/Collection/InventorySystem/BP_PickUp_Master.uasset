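; Master pickup actor for collectible plants, taking its mesh, material and type from the class defaults of its Plant class.
; The construction script applies the model and material to the static mesh.
; When BP_FirstPerson_Collector overlaps it, it adds the plant type enum to the Inventory in BP_GameInstance, marked as provisional.
; It then prints the result, plays dust and sound effects, and destroys itself.
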(event EventBeginPlay)

(event Collision|EventActorBeginOverlap
  (params (OtherActor :type Actor%20Object%20Reference))
  (bind _plant (Variables|Default|GetPlant))
  (bind _output (Utilities|ResolveSoftReference _plant))
  (bind _enumplanttype (Utilities|GetClassDefaults _output))
  (Utilities|Casting|CastToBP_FirstPerson_Collector OtherActor
    (:then
      (bind _asbp_game_instance (Utilities|Casting|CastToBP_GameInstance (Game|GetGameInstance)))
      (bind _returnvalue (Utilities|Array|Add (Variables|/Game/PracticeContent/Collection/InventorySystem/BP_GameInstance.BP_GameInstance_C|GetInventory _asbp_game_instance) _enumplanttype))
      (Development|PrintString (Utilities|String|Append (Utilities|String|Append (Utilities|String|Append "Added: " (Utilities|String|EnumtoString _enumplanttype)) " at position ") (Utilities|String|ToString(Integer) _returnvalue)))
      (Effects|SpawnEmitteratLocation "/Game/StarterContent/Particles/P_Ambient_Dust.P_Ambient_Dust" "0, 0, 0")
      (Audio|PlaySoundatLocation "/Game/Audio/pick-up.pick-up" (Transformation|GetWorldLocation (Variables|Default|GetStaticMesh)) "0, 0, 0" 1.0 1.0 0.0 0 0 0 0)
      (Actor|DestroyActor))
    (:CastFailed
      (Development|PrintText "Not player~"))))

(event EventTick
  (params (DeltaSeconds :type Float%20%28single-precision%29)))

(fn ConstructionScript
  (bind _plant (Variables|Default|GetPlant))
  (bind _staticmesh (Variables|Default|GetStaticMesh))
  (bind _output (Utilities|ResolveSoftReference _plant))
  (bind (_enumplanttype _plantstagemodels _growthstage _plantstagematerials _currentmodel _currentmaterial) (Utilities|GetClassDefaults _output))
  (Components|StaticMesh|SetStaticMesh _staticmesh _currentmodel)
  (Rendering|Material|SetMaterial _staticmesh 0 _currentmaterial))