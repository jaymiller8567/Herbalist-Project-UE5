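; BPC_Collector is a collector component that counts items picked up, stored in a folder for content no longer in use.
; The PickUp event increments Carrying and prints the new count for debugging.
; When Carrying equals Capacity, it clears CanPickUp and prints that capacity is reached.
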(event Custom|PickUp
  (bind _output_get (Variables|Default|SetCarrying (+ 1 (Variables|Default|GetCarrying))))
  (Development|PrintString (Utilities|String|Append "Carrying: " (Utilities|String|ToString(Integer) _output_get)))
  (if (== (Variables|Default|GetCarrying) (Variables|Default|GetCapacity))
    (Variables|Default|SetCanPickUp false)
    (Development|PrintString "Capacity Reached")))