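; BP_Book is an interactable book with an animated skeletal mesh and an overlap cube that detects BP_FirstPerson_Collector.
; Entering the cube shows a prompt widget, sets the ApproachBook flag and plays the open animation, which also plays on BeginPlay.
; Leaving hides the prompt and clears the flag.
; IA_Interact only prints a debug string while in range, and the close animation is never triggered.
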(event OnComponentBeginOverlap(InteractCube)
  (params (OverlappedComponent :type Primitive%20Component%20Object%20Reference) (OtherActor :type Actor%20Object%20Reference) (OtherComp :type Primitive%20Component%20Object%20Reference) (OtherBodyIndex :type Integer) (bFromSweep :type Boolean) (SweepResult :type Hit%20Result%20Structure%20%28by%20ref%29))
  (Utilities|Casting|CastToBP_FirstPerson_Collector OtherActor)
  (Development|SetHiddeninGame (Variables|Default|GetPromptWidget) false false)
  (Development|PrintString "Press E to open book!")
  (Variables|Default|SetApproachBook true)
  (Components|Animation|PlayAnimation (Variables|Default|GetSkeletalMesh) "/Game/ImportedModels/Book/Book_Open.Book_Open" false))

(event OnComponentEndOverlap(InteractCube)
  (params (OverlappedComponent :type Primitive%20Component%20Object%20Reference) (OtherActor :type Actor%20Object%20Reference) (OtherComp :type Primitive%20Component%20Object%20Reference) (OtherBodyIndex :type Integer))
  (Utilities|Casting|CastToBP_FirstPerson_Collector OtherActor)
  (Development|SetHiddeninGame (Variables|Default|GetPromptWidget) true false)
  (Development|PrintString "Player leaves  book!")
  (Variables|Default|SetApproachBook false))

(event Input|EnhancedActionEvents|EnhancedInputActionIA_Interact
  (params (ActionValue :type Boolean) (ElapsedSeconds :type Float%20%28double-precision%29) (TriggeredSeconds :type Float%20%28double-precision%29) (InputAction :type Input%20Action%20Object%20Reference :default "/Game/FirstPerson/Input/Actions/IA_Interact.IA_Interact"))
  (:Completed
    (if (Variables|Default|GetApproachBook)
      (Development|PrintString "Pressed E!"))))

(event EventBeginPlay
  (Components|Animation|PlayAnimation (Variables|Default|GetSkeletalMesh) "/Game/ImportedModels/Book/Book_Open.Book_Open" false))

(event EventTick
  (params (DeltaSeconds :type Float%20%28single-precision%29)))

(fn ConstructionScript)